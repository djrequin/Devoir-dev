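; Puzzle door Blueprint whose Cube snaps between a lowered and a raised relative position based on the IsOpened flag.
; On BeginPlay, the Cube is lowered if the door starts opened.
; The Switch event repositions the Cube from IsOpened, which it reads but does not change, then calls VerifyOpening on every linked Lamp.
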(event Custom|Switch
  (if (Variables|Default|GetIs_Opened%20?)
    (Transformation|SetRelativeLocation (Variables|Default|GetCube) "0.000000,0.000000,-140.000000" false false)
    (else
      (Transformation|SetRelativeLocation (Variables|Default|GetCube) "0.000000,0.000000,140.000000" false false)))
  (for _array_element (Variables|Default|GetLamp)
    (Default|VerifyOpening _array_element)))

(event EventBeginPlay
  (CallFunction|BeginInitialisation))

(fn ConstructionScript)

(fn BeginInitialisation
  (if (Variables|Default|GetIs_Opened%20?)
    (Transformation|SetRelativeLocation (Variables|Default|GetCube) "0.000000,0.000000,-140.000000" false false)))