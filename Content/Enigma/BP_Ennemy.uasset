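; Enemy Blueprint that can patrol or chase the player and shows a death screen on contact.
; Patrol moves to a random reachable point around itself, re-arming only on success, while CanMove repeatedly re-issues AIMoveTo toward the player on success or failure.
; Box overlap with the player creates the death widget once if the CanMove flag is set.
; StopMove is empty, and its likely stop logic sits disconnected.
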(event OnComponentBeginOverlap(Box)
  (params (OverlappedComponent :type Primitive%20Component%20Object%20Reference) (OtherActor :type Actor%20Object%20Reference) (OtherComp :type Primitive%20Component%20Object%20Reference) (OtherBodyIndex :type Integer) (bFromSweep :type Boolean) (SweepResult :type Hit%20Result%20Structure%20%28by%20ref%29))
  (Utilities|Casting|CastToBP_ThirdPersonCharacter OtherActor)
  (if (Variables|Default|GetCan_Move_)
    (Utilities|FlowControl|DoOnce false
      (:Completed
        (bind _returnvalue (UserInterface|CreateWidget "/Game/UI/WB_Death_Screen.WB_Death_Screen_C"))
        (UserInterface|Viewport|AddtoViewport _returnvalue 0)))))

(event Custom|Patrol
  (Utilities|FlowControl|DoOnce false :!label _label
    (:Completed
      (AI|AIMoveTo self (.RandomLocation (AI|Navigation|GetRandomReachablePointinRadius (Transformation|GetWorldLocation (Variables|Collision|GetCapsuleComponent)) (Variables|Default|GetPatrol_Radius) 0 0)) 0 5.0 false
        (:OnSuccess
          (goto _label Reset))))))

(event EventBeginPlay)

(event EventCanMove
  (bind _asbp_third_person_character (Utilities|Casting|CastToBP_ThirdPersonCharacter (Game|GetPlayerCharacter 0) :!label _label))
  (AI|AIMoveTo self "0, 0, 0" _asbp_third_person_character 5.0 false
    (:OnSuccess
      (goto _label))
    (:OnFail
      (goto _label))))

(event EventStopMove)

(fn ConstructionScript)